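; Patrol route actor that supplies successive world-space locations along a spline for back-and-forth patrolling.
; Each GetPatrolPointLocation call first advances PatrolIndex by Direction, then returns that spline point's location, so querying also changes state.
; Direction flips to backward when the index reaches the point count, one past the last valid index, and to forward at zero or below.
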(event Custom|Increment%20Patrol%20Point%20Index
  (Variables|Default|SetPatrolIndex (+ (Variables|Default|GetPatrolIndex) (Variables|Default|GetDirection)))
  (if (>= (Variables|Default|GetPatrolIndex) (Spline|GetNumberOfSplinePoints (Variables|Default|GetSpline))) ; if at end, reverse
    ;[1 1 1] Flip the direction
    (Variables|Default|SetDirection -1)
    (elif (<= (Variables|Default|GetPatrolIndex) 0) ; if at beginning, start over
      (Variables|Default|SetDirection 1))))

(fn ConstructionScript)

(fn GetPatrolPointLocation
  (CallFunction|IncrementPatrolPointIndex)
  (return (Spline|GetLocationatSplinePoint (Variables|Default|GetSpline) (Variables|Default|GetPatrolIndex) "World")))