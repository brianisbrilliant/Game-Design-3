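; Base enemy character for the behavior tree AI, with a zombie melee attack and a toggleable fire effect on its right hand.
; Attack plays a montage and calls the OnAttackEnd dispatcher whether it completes or is interrupted.
; SpawnFire creates and attaches BP_Fire once, then reuses it by raising its Niagara spawn rate.
; ExtinguishFire zeroes that rate so remaining particles fade naturally instead of destroying the actor.
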(event Custom|Attack
  ;[1 1 1] Attack plays an animation and calls an event dispatcher to run after it is completed.
  (Animation|Montage|PlayMontage (Variables|Character|GetMesh) "/Game/BSP_ZombieAnims/Animations/Standing/Attack/AS_NAAT_Zombie_Attack_RH_Stand_Montage.AS_NAAT_Zombie_Attack_RH_Stand_Montage"
    (:OnCompleted
      _)
    (:OnInterrupted
      _))
  (Default|CallOnAttackEnd))

(event Custom|SpawnFire
  ;[1 1 1] if the fire exists, just change it's spawn rate to 1111 to turn it on.
  ; otherwise, create it.
  (bind _fire (Variables|Default|GetFire)
    (:then
      (Niagara|SetNiagaraVariable(Float) (Variables|/Game/Blueprints/BP_Fire.BP_Fire_C|GetNiagara _fire) "SpawnRate" 1111.0))
    (:else
      (bind _returnvalue (Game|SpawnActorfromClass "/Game/Blueprints/BP_Fire.BP_Fire_C" (Transformation|GetActorTransform) "Undefined" "MultiplyWithRoot" 0 0))
      (bind _output_get (Variables|Default|SetFire _returnvalue)) ; promote to variable
      (Transformation|AttachComponentToComponent _output_get (Variables|Character|GetMesh) "hand_rSocket" "SnapToTarget" "SnapToTarget" "SnapToTarget" true)
      (Variables|Default|SetFireIsSpawned true))))

(event Custom|Extinguish%20Fire
  (Variables|Default|GetFire
    (:then
      ;[1 1 1] Don't turn it off, just set the spawn rate to 0. This allows the remaining particles to smoothly disappear
      (Niagara|SetNiagaraVariable(Float) (Variables|/Game/Blueprints/BP_Fire.BP_Fire_C|GetNiagara (Variables|Default|GetFire)) "SpawnRate" 0.0)
      (Variables|Default|SetFireIsSpawned false))
    (:else)))

(event EventBeginPlay
  ;[1 1 1] Begin Play Does Nothing.
  ; The AI Controller is set in the class settings under "AI Controller"
  (Development|PrintString "ai begin play"))

(fn ConstructionScript)