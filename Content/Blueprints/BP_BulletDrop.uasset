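; BP_BulletDrop is a test Blueprint that compares a hand-rolled bullet-drop calculation against Unreal's built-in PredictProjectilePath, redrawing both from an Arrow component every 1.2 seconds.
; The custom event steps along the arc by SimFrequency, line-tracing and drawing debug segments until a hit or the loop ends, then resets.
; A half-step gravity offset on the first segment aims to match the prediction, though only X velocity is divided by frequency.
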(event Custom|Really%20Cool%20Bullet%20Drop%20Calculator
  (Variables|Default|SetVelocity (+ (Variables|Default|GetVelocity) (Math|Vector|MakeVector 0.0 0.0 (* (/ -9.8e+02 (Math|Float|Square (Variables|Default|GetSim%20Frequency))) 0.5))))
  (Variables|Default|SetEnd (+ (Variables|Default|GetStart) (/ (Variables|Default|GetVelocity) (Math|Vector|MakeVector (Variables|Default|GetSim%20Frequency) 1.0 1.0))))
  (Utilities|FlowControl|ForLoopwithBreak 1 (Math|Float|Truncate (Variables|Default|GetSim%20Frequency)) :!label _label ; break if the line trace hits something
    (:LoopBody
      (Rendering|Debug|DrawDebugLine (Variables|Default|GetStart) (Variables|Default|GetEnd) "(R=1.000000,G=0.000000,B=0.774170,A=1.000000)" (Variables|Default|GetMax%20Sim%20Time) 0.0)
      (Rendering|Debug|DrawDebugSphere (Variables|Default|GetEnd) 5.0 12 "(R=0.000000,G=0.706227,B=1.000000,A=1.000000)" (Variables|Default|GetMax%20Sim%20Time) 0.5)
      (bind _returnvalue (Class|KismetSystemLibrary|LineTraceSinglebyProfile (Variables|Default|GetStart) (Variables|Default|GetEnd) "BlockAll" false 0 "ForDuration" true))
      (if _returnvalue
        (Development|PrintString "We hit something!")
        (goto _label Break)
        (else
          (Variables|Default|SetStart (Variables|Default|GetEnd)) ; set the new start location
          ;[1 1 1] Add gravity to velocity.
          (Variables|Default|SetVelocity (+ (Variables|Default|GetVelocity) (Math|Vector|MakeVector 0.0 0.0 (/ -9.8e+02 (Math|Float|Square (Variables|Default|GetSim%20Frequency))))))
          ;[1 1 1] Set end to the NEW start position plus velocity
          (Variables|Default|SetEnd (+ (Variables|Default|GetStart) (/ (Variables|Default|GetVelocity) (Math|Vector|MakeVector (Variables|Default|GetSim%20Frequency) 1.0 1.0)))))))
    (:Completed
      ;[1 1 1] from the for loop's Completed...reset start and velocity when complete
      (Variables|Default|SetStart (Transformation|GetWorldLocation (Variables|Default|GetArrow)))
      (Variables|Default|SetVelocity (Variables|Default|Getstartingvelocity)))))

(event EventBeginPlay
  (bind _arrow (Variables|Default|GetArrow))
  (bind _returnvalue (Transformation|GetWorldLocation _arrow))
  (Variables|Default|SetStart _returnvalue)
  (Utilities|FlowControl|Sequence :!label _label
    (:then_0
      (CallFunction|ReallyCoolBulletDropCalculator))
    (:then_1
      (Class|GameplayStatics|BlueprintPredictProjectilePathAdvanced (Utilities|Struct|MakePredictProjectilePathParams _returnvalue (Variables|Default|Getstartingvelocity) true 0.0 (Variables|Default|GetMax%20Sim%20Time) true "ECC_WorldStatic" "ObjectTypeQuery1" 0 (Variables|Default|GetSim%20Frequency) 0.0 "ForDuration" 1.0 false))
      (Utilities|FlowControl|Delay 1.2)
      (goto _label))))

(fn ConstructionScript)