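; BP_CameraDoor is a door that shows itself opening by temporarily taking over the player's camera.
; OpenDoor records the door in the game mode's LevelData open-doors list, blends the view to it, lowers it with a timeline, then blends to the passed-in target after a pause.
; quietOpen moves the door without the camera shot, through a DoOnce that resetthing re-arms.
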(event Custom|OpenDoor
  (params (NewViewTarget :type Actor%20Object%20Reference))
  ;[1 0.3362 0.2196] Add this door to the array of open doors in the save game
  (bind _asbp_third_person_game_mode (Utilities|Casting|CastToBP_ThirdPersonGameMode (Game|GetGameMode)))
  (Utilities|Array|AddUnique (Variables|/Game/Blueprints/Saves/SG_LevelData.SG_LevelData_C|GetOpenDoors (Variables|/Game/ThirdPerson/Blueprints/BP_ThirdPersonGameMode.BP_ThirdPersonGameMode_C|GetLevel%20Data _asbp_third_person_game_mode)) self)
  (Game|Player|SetViewTargetwithBlend (Game|GetPlayerController 0) self (Variables|Default|GetBlend%20Time) "VTBlend_Cubic" 0.0 true)
  (Utilities|FlowControl|Delay (Variables|Default|GetBlend%20Time))
  (bind _newtrack_0 (Timeline|Timeline Play)
    (:Update
      (Transformation|SetRelativeLocation (Variables|Default|GetDoor) (Math|Vector|Lerp(Vector) "0.000000,0.000000,150.000000" "0.000000,0.000000,-130.000000" _newtrack_0) false false))
    (:Finished
      (Utilities|FlowControl|Delay 2.0) ; waiting 2 seconds while the door opens
      (Game|Player|SetViewTargetwithBlend (Game|GetPlayerController 0) NewViewTarget (/ (Variables|Default|GetBlend%20Time) 2.0) "VTBlend_Cubic" 0.0 false) ; shift camera back to player
    )))

(event Custom|quietOpen
  (Utilities|FlowControl|DoOnce false
    (:Completed
      (bind _newtrack_0 (Timeline|Timeline_0 Play)
        (:Update
          (Transformation|SetRelativeLocation (Variables|Default|GetDoor) (Math|Vector|Lerp(Vector) "0.000000,0.000000,150.000000" "0.000000,0.000000,-130.000000" _newtrack_0) false false))))))

(event Custom|reset%20thing
  (Utilities|FlowControl|DoOnce false) ; enters at Reset
)

(fn ConstructionScript)