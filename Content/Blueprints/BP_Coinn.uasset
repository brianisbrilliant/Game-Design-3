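; Collectible coin actor that the third-person character picks up on mesh overlap, with collection recorded per level.
; A first pickup adds the coin's own actor reference uniquely to the level coin save held by GM_CollectingCoins, then destroys it.
; LoadCollectedState flags a coin as already collected and swaps in the collected material; such coins are destroyed on overlap without being recorded again.
; An invalid save only prints an error, leaving the coin in place.
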(event OnComponentBeginOverlap(StaticMesh)
  (params (OverlappedComponent :type Primitive%20Component%20Object%20Reference) (OtherActor :type Actor%20Object%20Reference) (OtherComp :type Primitive%20Component%20Object%20Reference) (OtherBodyIndex :type Integer) (bFromSweep :type Boolean) (SweepResult :type Hit%20Result%20Structure%20%28by%20ref%29))
  (Utilities|Casting|CastToBP_ThirdPersonCharacter OtherActor)
  (if (Variables|Default|GetHasBeenCollected)
    (Actor|DestroyActor :!label _label)
    (else
      (bind _asgm_collecting_coins (Utilities|Casting|CastToGM_CollectingCoins (Game|GetGameMode)))
      (Utilities|IsValid (Variables|/Game/Blueprints/NewSaves/GM_CollectingCoins.GM_CollectingCoins_C|GetLevelCoinSave _asgm_collecting_coins)
        (:Is%20Valid
          (Utilities|Array|AddUnique (Variables|/Game/Blueprints/NewSaves/SG_LevelCollectedCoins.SG_LevelCollectedCoins_C|GetSavedCollectedCoins (Variables|/Game/Blueprints/NewSaves/GM_CollectingCoins.GM_CollectingCoins_C|GetLevelCoinSave _asgm_collecting_coins)) self)
          (goto _label))
        (:Is%20Not%20Valid
          (Development|PrintString "LEVEL SAVE NOT VALID" true true "(R=0.000000,G=0.660000,B=1.000000,A=1.000000)" 5.0))))))

(event Custom|Load%20Collected%20State
  (Variables|Default|SetHasBeenCollected true)
  (Rendering|Material|SetMaterial (Variables|Default|GetStaticMesh) 0 "/Game/Materials/MI_CollectedCoin.MI_CollectedCoin")
  (Development|PrintString "Collected State Loadedd"))

(fn ConstructionScript)