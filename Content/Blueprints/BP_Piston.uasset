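; BP_Piston is an animated piston that moves up and down with sound, rumble and camera shake.
; On BeginPlay it starts a timeline with a random time offset, which drives the piston's relative Z position.
; The timeline's Thud event plays a randomly pitched, quiet hit sound, force feedback and a source-based camera shake for the first player.
; Older shake and feedback nodes remain unconnected.
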(event EventBeginPlay
  (Utilities|FlowControl|Sequence
    (:then_0
      (bind _newtrack_0 (Timeline|Timeline Play)
        (:Update
          (Transformation|SetRelativeLocation (Variables|Default|GetPiston) (Math|Vector|MakeVector 0.0 0.0 (- (* _newtrack_0 4e+01) 2e+01)) false false))
        (:Thud
          (Audio|SpawnSoundatLocation "/Game/Audio/HitHurt5OneShot.HitHurt5OneShot" (Transformation|GetWorldLocation (Variables|Default|GetPiston)) "0, 0, 0" (Math|Random|RandomFloatinRange 0.0 0.3) (Math|Random|RandomFloatinRange 0.01 0.2) 0.0 0 0)
          (Audio|Components|Audio|Play (Variables|Default|GetForceFeedback) 0.0)
          (Class|PlayerController|ClientStartCameraShakefromSource (Game|GetPlayerController 0) "/Game/Blueprints/CameraShakes/CS_Piston.CS_Piston_C" (Variables|Default|GetCameraShakeSource)))))
    (:then_1
      (Timeline|Timeline SetNewTime))))

(fn ConstructionScript)