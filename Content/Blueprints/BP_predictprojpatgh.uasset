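; Debug test actor that compares a hand-rolled bullet-drop trajectory with Unreal's Predict Projectile Path, both launched from an Arrow along world X.
; The custom event steps velocity with a gravity term, drawing lines and spheres without collision, while the built-in prediction traces the Pawn channel.
; BeginPlay repeats both through a Delay loop, raising BulletSpeed as it goes.
; Tick calls an empty bullet-drop stub.
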(event Custom|Brian's%20Custom%20Trace%20WithDraop
  (bind _predict_params_sim_frequency (Variables|Default|GetPredict%20Params%20Sim%20Frequency))
  (bind _returnvalue (/ 1.0 _predict_params_sim_frequency))
  (bind _output_get (Variables|Default|SetStart (Transformation|GetWorldLocation (Variables|Default|GetArrow)))) ; start at arrow
  (bind _output_get_2 (Variables|Default|SetVelocity (Math|Vector|MakeVector (* (Variables|Default|GetBulletSpeed) (/ 1.0 (Variables|Default|GetPredict%20Params%20Sim%20Frequency))) 0.0 0.0)))
  (Variables|Default|SetEnd (+ _output_get _output_get_2))
  (for _index (range 0 (Math|Float|Truncate (* (Variables|Default|GetPredict%20Params%20Max%20Sim%20Time) (Variables|Default|GetPredict%20Params%20Sim%20Frequency)))) ; run 10 times, for .1 seconds. a total of 1 second.
    (Rendering|Debug|DrawDebugLine (Variables|Default|GetStart) (Variables|Default|GetEnd) "(R=1.000000,G=0.000000,B=0.694110,A=1.000000)" (Variables|Default|GetDebugDuration) 0.0)
    (Rendering|Debug|DrawDebugSphere (Variables|Default|GetEnd) 1e+01 12 "(R=0.000000,G=0.521003,B=1.000000,A=1.000000)" (Variables|Default|GetDebugDuration))
    (Variables|Default|SetStart (Variables|Default|GetEnd))
    (bind _output_get_3 (Variables|Default|SetVelocity (Math|Vector|MakeVector (.x (Variables|Default|GetVelocity)) (.y (Variables|Default|GetVelocity)) (+ (.z (Variables|Default|GetVelocity)) (* 0.5 -98.0 _returnvalue)))))
    (Variables|Default|SetEnd (+ (Variables|Default|GetStart) (Variables|Default|GetVelocity)))
    (Development|PrintString (Utilities|String|Append "time step" (Utilities|String|ToString(Float) _returnvalue) "  velocity " (Utilities|String|ToString(Vector) _output_get_3)))))

(event EventBeginPlay
  (Utilities|FlowControl|Sequence :!label _label
    (:then_0
      (CallFunction|Brian'sCustomTracewithDraop))
    (:then_1
      (Class|GameplayStatics|BlueprintPredictProjectilePathAdvanced (Utilities|Struct|MakePredictProjectilePathParams (Transformation|GetWorldLocation (Variables|Default|GetArrow)) (Math|Vector|MakeVector (Variables|Default|GetBulletSpeed) 0.0 0.0) true 0.0 (Variables|Default|GetPredict%20Params%20Max%20Sim%20Time) true "ECC_Pawn" "ObjectTypeQuery1" 0 (Variables|Default|GetPredict%20Params%20Sim%20Frequency) 0.0 "ForDuration" 1.0 true))))
  (bind _output_get (Variables|Default|SetBulletSpeed (+ (Variables|Default|GetBulletSpeed) 5e+01)))
  (Development|PrintString (Utilities|String|ToString(Float) _output_get))
  (Utilities|FlowControl|Delay 1.0)
  (goto _label))

(event Collision|EventActorBeginOverlap
  (params (OtherActor :type Actor%20Object%20Reference)))

(event EventTick
  (params (DeltaSeconds :type Float%20%28single-precision%29))
  (CallFunction|Tickedoffbulletdropp DeltaSeconds))

(fn ConstructionScript)

(fn Tickedoffbulletdropp
  (params (Event%20Tick :type Float%20%28double-precision%29))
  (if (LocalVariables|GetisActive)
    _))