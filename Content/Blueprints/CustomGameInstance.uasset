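; Game instance that saves, loads and deletes player progress and per-level pickup data.
; On init it loads or creates an SG_LevelData save keyed by the current level name, held for coins to update as collected.
; Player save and load copy stamina, transform and shoot/sprint abilities via SG_Coding2 in a separate slot, and also trigger the level save or load.
; Deleting clears both slots, then reopens the level if the level slot was removed.
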(event Custom|Delete%20Save%20Data
  (bind _returnvalue (SaveGame|DeleteGameinSlot (Variables|Default|GetSlotName))) ; Delete Player Data
  (if _returnvalue
    _
    (else
      (Development|PrintString "could not delete player save")))
  (bind _returnvalue_2 (Game|GetCurrentLevelName true))
  (bind _returnvalue_3 (SaveGame|DeleteGameinSlot _returnvalue_2)) ; Delete Current Level's Data
  (if _returnvalue_3
    (Development|PrintString "successfully deleted saves")
    (bind _returnvalue_4 (Game|GetCurrentLevelName true))
    (Game|OpenLevel(byName) (Utilities|String|StringToName _returnvalue_4))
    (else
      (Development|PrintString "could not delete level save"))))

(event Custom|SavePlayer
  (Development|PrintString "Saving game from game instance")
  (CallFunction|SaveLevel)
  (bind _returnvalue (SaveGame|DoesSaveGameExist (Variables|Default|GetSlotName)))
  (if _returnvalue
    (bind _returnvalue_2 (SaveGame|LoadGamefromSlot (Variables|Default|GetSlotName)))
    (bind _assg_coding_2 (Utilities|Casting|CastToSG_Coding2 _returnvalue_2))
    (Variables|Default|SetPlayerData _assg_coding_2)
    (else
      (bind _returnvalue_3 (SaveGame|CreateSaveGameObject "/Game/Blueprints/SG_Coding2.SG_Coding2_C"))
      (Variables|Default|SetPlayerData _returnvalue_3)))
  ;[0.2906 0.2906 0.2906 1 32] Save Data
  (bind _asbp_third_person_character (Utilities|Casting|CastToBP_ThirdPersonCharacter (Game|GetPlayerCharacter 0)))
  (Variables|/Game/Blueprints/SG_Coding2.SG_Coding2_C|SetPlayerStamina (Variables|Default|GetPlayerData) (Variables|/Game/ThirdPerson/Blueprints/BP_ThirdPersonCharacter.BP_ThirdPersonCharacter_C|GetStamina _asbp_third_person_character))
  (Variables|/Game/Blueprints/SG_Coding2.SG_Coding2_C|SetPlayerTransform (Variables|Default|GetPlayerData) (Transformation|GetWorldTransform (Variables|/Script/Engine.Character|GetCapsuleComponent _asbp_third_person_character)))
  (Variables|/Game/Blueprints/SG_Coding2.SG_Coding2_C|SetPlayerCanShoot (Variables|Default|GetPlayerData) (Variables|/Game/ThirdPerson/Blueprints/BP_ThirdPersonCharacter.BP_ThirdPersonCharacter_C|GetCanShoot _asbp_third_person_character))
  (Variables|/Game/Blueprints/SG_Coding2.SG_Coding2_C|SetPlayerCanSprint (Variables|Default|GetPlayerData) (Variables|/Game/ThirdPerson/Blueprints/BP_ThirdPersonCharacter.BP_ThirdPersonCharacter_C|GetCanSprint _asbp_third_person_character))
  (SaveGame|SaveGametoSlot (Variables|Default|GetPlayerData) (Variables|Default|GetSlotName)))

(event Custom|LoadPlayer
  (bind _slotname (Variables|Default|GetSlotName))
  (Development|PrintString "Loading game from game instance")
  (CallFunction|LoadLevel)
  (Development|PrintString "Load game")
  (bind _returnvalue (SaveGame|DoesSaveGameExist _slotname))
  (if _returnvalue
    (bind _returnvalue_2 (SaveGame|LoadGamefromSlot _slotname))
    (bind _assg_coding_2 (Utilities|Casting|CastToSG_Coding2 _returnvalue_2))
    (bind _asbp_third_person_character (Utilities|Casting|CastToBP_ThirdPersonCharacter (Game|GetPlayerCharacter 0)))
    (Variables|/Game/ThirdPerson/Blueprints/BP_ThirdPersonCharacter.BP_ThirdPersonCharacter_C|SetCanSprint _asbp_third_person_character (Variables|/Game/Blueprints/SG_Coding2.SG_Coding2_C|GetPlayerCanSprint _assg_coding_2))
    (Variables|/Game/ThirdPerson/Blueprints/BP_ThirdPersonCharacter.BP_ThirdPersonCharacter_C|SetCanShoot _asbp_third_person_character (Variables|/Game/Blueprints/SG_Coding2.SG_Coding2_C|GetPlayerCanShoot _assg_coding_2))
    (Transformation|SetWorldTransform (Variables|/Script/Engine.Character|GetCapsuleComponent _asbp_third_person_character) (Variables|/Game/Blueprints/SG_Coding2.SG_Coding2_C|GetPlayerTransform _assg_coding_2) false false)
    (Variables|/Game/ThirdPerson/Blueprints/BP_ThirdPersonCharacter.BP_ThirdPersonCharacter_C|SetStamina _asbp_third_person_character (Variables|/Game/Blueprints/SG_Coding2.SG_Coding2_C|GetPlayerStamina _assg_coding_2))))

(event Custom|SaveLevel
  (Development|PrintString "Saving Level From Game Instance" true true "(R=0.169946,G=0.025023,B=1.000000,A=1.000000)")
  (bind _returnvalue (Game|GetCurrentLevelName true))
  (SaveGame|SaveGametoSlot (Variables|Default|GetLevel%20Data) _returnvalue) ; the Level Dataa will be updated \neach time a coin is collected
)

(event Custom|LoadLevel
  (Development|PrintString "Loading Level from Game instance" true true "(R=0.171441,G=0.025187,B=1.000000,A=1.000000)")
  (bind _returnvalue (Game|GetCurrentLevelName true))
  (bind _returnvalue_2 (SaveGame|DoesSaveGameExist _returnvalue))
  (if _returnvalue_2
    (Default|LoadCollectedPickups (Variables|Default|GetLevel%20Data))))

(event EventInit
  ;[0.1823 0.4736 1] Creating the Level Data Variable, so that the coins can talk to it
  (bind _returnvalue (Game|GetCurrentLevelName true))
  (bind _returnvalue_2 (SaveGame|DoesSaveGameExist _returnvalue))
  (if _returnvalue_2
    (bind _returnvalue_3 (SaveGame|LoadGamefromSlot _returnvalue)) ; create your parameter from this node
    (bind _assg_level_data (Utilities|Casting|CastToSG_LevelData _returnvalue_3))
    (Variables|Default|SetLevel%20Data _assg_level_data) ; As SG Level Data
    (else
      (bind _returnvalue_4 (SaveGame|CreateSaveGameObject "/Game/Blueprints/Saves/SG_LevelData.SG_LevelData_C"))
      (Variables|Default|SetLevel%20Data _returnvalue_4))))