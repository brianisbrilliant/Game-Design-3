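; BP_DialogSystem is a test dialogue player that steps through the lines of the DT_TestDialogue data table on screen.
; Shortly after BeginPlay it creates the W_DataTableDialogue widget and starts DebugSystem.
; DebugSystem writes the current row's text into the widget, waits, increments RowIndex and calls itself until a row lookup fails.
; The NextLine event is an empty stub, so lines advance only on the timed delay.
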(event Custom|NextLine)

(event Custom|debug%20system
  (Development|PrintString "Starting Debug Systtem")
  (bind _outrownames (DataTable|GetDataTableRowNames "/Game/Blueprints/DT_Dialogue/DT_TestDialogue.DT_TestDialogue"))
  (bind _returnvalue (Utilities|GetDataTableRow "/Game/Blueprints/DT_Dialogue/DT_TestDialogue.DT_TestDialogue" (Utilities|Array|Get(acopy) _outrownames (Variables|Default|GetRow%20Index)))
    (:then
      (Rendering|Components|TextRender|SetText (Variables|/Game/Blueprints/DT_Dialogue/W_DataTableDialogue.W_DataTableDialogue_C|GetTextBlock_0 (stale EventBeginPlay _output_get)) (.text _returnvalue))
      (Utilities|FlowControl|Delay 2.0)
      (Math|Integer|IncrementInt (Variables|Default|GetRow%20Index)
        (:%20%20
          (CallFunction|DebugSystem))))
    (:RowNotFound
      (Development|PrintString "Row Not Fount"))))

(event EventBeginPlay
  (Utilities|FlowControl|Delay 2.0)
  (bind _returnvalue (UserInterface|CreateWidget "/Game/Blueprints/DT_Dialogue/W_DataTableDialogue.W_DataTableDialogue_C"))
  (bind _output_get (Variables|Default|SetW_Dialogue _returnvalue))
  (UserInterface|Viewport|AddtoViewport _output_get 0)
  (CallFunction|DebugSystem))

(fn ConstructionScript)