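; Base enemy character Blueprint providing sword combat actions, a patrol route getter and movement speed presets.
; WieldSword spawns a sword actor attached to the right-hand socket, while SheathSword fires a dispatcher and destroys it, both updating a wielding flag.
; Attack plays a slash montage and fires OnAttackEnd whether it completes or is interrupted.
; SetMovementSpeed maps an enum to max walk speed but always returns zero.
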(event Custom|Attack
  (Animation|Montage|PlayMontage (Variables|Character|GetMesh) "/Game/Animations/Melee/migrate/Montage_Sword_Slash.Montage_Sword_Slash"
    (:OnCompleted
      _)
    (:OnInterrupted
      _))
  (Default|CallOnAttackEnd))

(event Custom|WieldSword
  (bind _returnvalue (Game|SpawnActorfromClass "/Game/Blueprints/Enemy_Ali/Weapons/BP_Sword.BP_Sword_C" (Transformation|GetActorTransform) "Undefined" "MultiplyWithRoot" 0 0))
  (Variables|Default|SetSword%20Actor _returnvalue)
  (Transformation|AttachComponentToComponent _returnvalue (Variables|Character|GetMesh) "hand_rSword_Socket" "SnapToTarget" "SnapToTarget" "SnapToTarget" true)
  (Variables|Default|SetIsWieldingSword true))

(event Custom|Sheath%20Sword
  (Default|CallOnSheathSword)
  (Actor|DestroyActor (Variables|Default|GetSword%20Actor))
  (Variables|Default|SetIsWieldingSword false))

(event EventBeginPlay
  (Development|PrintString "Starting begin play "))

(fn ConstructionScript)

(fn GetPatrolRoute
  (return (Variables|AI|GetPatrolRoute)))

(fn SetMovementSpeed
  (params (Speed :type E_MovementSpeed%20Enum :default "NewEnumerator0"))
  (Variables|/Script/Engine.CharacterMovementComponent|SetMaxWalkSpeed (Variables|Character|GetCharacterMovement) (Utilities|Select :Index Speed :NewEnumerator0 0.0 :NewEnumerator1 1.5e+02 :NewEnumerator2 3e+02 :NewEnumerator3 5e+02))
  (return 0.0))