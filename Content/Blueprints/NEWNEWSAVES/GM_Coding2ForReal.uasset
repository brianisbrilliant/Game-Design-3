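; Game mode that manages per-level save data, using the current level name as the save slot.
; On BeginPlay it loads or creates an SG_LevelSave, restores collected coins and open doors, and moves the player to any non-origin saved location.
; Checkpoint stores a player transform and FinishedLevel clears it, both then writing the slot via SaveGame.
; A save that fails the cast is deleted, with no replacement created in that run.
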(event Custom|Save%20Game
  (bind _returnvalue (Game|GetCurrentLevelName true))
  (bind _returnvalue_2 (SaveGame|SaveGametoSlot (Variables|Default|GetLevel%20Save) _returnvalue))
  (if _returnvalue_2
    (Development|PrintString "Saved level")
    (else
      (Development|PrintString "Could not Save Level"))))

(event EventBeginPlay
  (Development|PrintString "Loaded into the GM_Coding2ForReal Game Mode" true true "(R=1.000000,G=0.000000,B=0.028497,A=1.000000)" 2e+01)
  ;[1 1 1] Is there a level save file for this level's name? If not, create one, so that we can start editing it.
  ; if there is - load it and store it to the "Level Save" variable, so we can start editing it.
  (bind _returnvalue (Game|GetCurrentLevelName true))
  (bind _returnvalue_2 (SaveGame|DoesSaveGameExist _returnvalue))
  (if _returnvalue_2
    (bind _returnvalue_3 (SaveGame|LoadGamefromSlot _returnvalue))
    (bind _assg_level_save (Utilities|Casting|CastToSG_LevelSave _returnvalue_3)
      (:then
        (bind _output_get (Variables|Default|SetLevel%20Save _assg_level_save))
        (Default|LoadCollectedCoins _output_get) ; change the coins that have \nalready been collected.
        (Default|LoadOpenDoors _output_get)
        (if (not (Class|KismetMathLibrary|EqualExactlyVectorVector (.location (Variables|/Game/Blueprints/NEWNEWSAVES/SG_LevelSave.SG_LevelSave_C|GetPlayerTransform (Variables|Default|GetLevel%20Save))) "0, 0, 0")) ; If the value of player transform is NOT 0,0,0,\nmove them to that spot.
          (Transformation|SetWorldTransform (Variables|/Script/Engine.Character|GetCapsuleComponent (Game|GetPlayerCharacter 0)) (Variables|/Game/Blueprints/NEWNEWSAVES/SG_LevelSave.SG_LevelSave_C|GetPlayerTransform (Variables|Default|GetLevel%20Save)) false false)))
      (:CastFailed
        (Development|PrintString "Cast to SG_Level Save Failed, deleting")
        (SaveGame|DeleteGameinSlot _returnvalue) ; Delete the old saves from different \nsave game types
      ))
    (else
      (bind _returnvalue_4 (SaveGame|CreateSaveGameObject "/Game/Blueprints/NEWNEWSAVES/SG_LevelSave.SG_LevelSave_C"))
      (Variables|Default|SetLevel%20Save _returnvalue_4)
      (Development|PrintString "Created new SG_Level Save"))))

(fn ConstructionScript)

(fn Checkpoint
  (params (PlayerTransform :type Transform))
  (Variables|/Game/Blueprints/NEWNEWSAVES/SG_LevelSave.SG_LevelSave_C|SetPlayerTransform (Variables|Default|GetLevel%20Save) PlayerTransform) ; set the Player Transform var\non the Level Save
  (CallFunction|SaveGame))

(fn FinishedLevel
  (Variables|/Game/Blueprints/NEWNEWSAVES/SG_LevelSave.SG_LevelSave_C|SetPlayerTransform (Variables|Default|GetLevel%20Save) "") ; Reset player start location to 0,0,0
  (CallFunction|SaveGame))