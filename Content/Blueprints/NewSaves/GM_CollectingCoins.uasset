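; GM_CollectingCoins is a game mode Blueprint that manages a per-level save of collected coins.
; On BeginPlay it loads the save slot named after the current level and calls LoadCollectedCoins, or creates a new SG_LevelCollectedCoins object if no slot exists.
; Its SaveGame event writes the held LevelCoinSave object back to that level-named slot, with debug prints reporting progress and failures.
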(event Custom|Save%20Game
  (bind _returnvalue (Game|GetCurrentLevelName true))
  (bind _returnvalue_2 (SaveGame|SaveGametoSlot (Variables|Default|GetLevelCoinSave) _returnvalue))
  (if _returnvalue_2
    (Development|PrintString "GameSaved!")
    (else
      (Development|PrintString "Game NOT saved"))))

(event EventBeginPlay
  (Development|PrintString "Starting GM CollecingCoins")
  (bind _returnvalue (Game|GetCurrentLevelName true))
  (bind _returnvalue_2 (SaveGame|DoesSaveGameExist _returnvalue))
  (if _returnvalue_2
    (Development|PrintString "Loading game from slot")
    (bind _returnvalue_3 (SaveGame|LoadGamefromSlot _returnvalue))
    (bind _assg_level_collected_coins (Utilities|Casting|CastToSG_LevelCollectedCoins _returnvalue_3)
      (:then
        (Variables|Default|SetLevelCoinSave _assg_level_collected_coins)
        (Default|LoadCollectedCoins _assg_level_collected_coins))
      (:CastFailed
        (Development|PrintString "failed to cast to SG_levelcollectedcoins")))
    (else
      (Development|PrintString "creating a new save game")
      (bind _returnvalue_4 (SaveGame|CreateSaveGameObject "/Game/Blueprints/NewSaves/SG_LevelCollectedCoins.SG_LevelCollectedCoins_C"))
      (Variables|Default|SetLevelCoinSave _returnvalue_4))))

(fn ConstructionScript)