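; Data structures and algorithms sandbox Blueprint that visualizes indexed nodes as a row of debug spheres.
; A loop from zero to LastIndex spaces the spheres along X and blends their color from red to blue by index.
; BeginPlay enters the Shownodes chain, which re-calls itself after a delay one second longer than Duration, so the row repeatedly appears and vanishes.
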(event Custom|Show%20nodes
  (bind _last_index (Variables|Default|GetLast%20Index))
  (bind _duration (Variables|Default|GetDuration))
  (for _index (range 0 _last_index)
    (Rendering|Debug|DrawDebugSphere (Math|Vector|MakeVector (Math|Conversions|ToFloat(Integer) (* _index 222)) 0.0 2e+02) 111.0 12 (Math|Color|Lerp(LinearColor) "(R=1.000000,G=0.070127,B=0.000000,A=1.000000)" "(R=0.000000,G=0.070262,B=1.000000,A=1.000000)" (/ (Math|Conversions|ToFloat(Integer) _index) (Math|Conversions|ToFloat(Integer) _last_index))) _duration 2.0))
  (Utilities|FlowControl|Delay (+ _duration 1.0))
  (CallFunction|ShowNodes) ; This is a GOTO lol
)

(event EventBeginPlay
  (bind _last_index (Variables|Default|GetLast%20Index))
  (bind _duration (Variables|Default|GetDuration))
  (for _index (range 0 _last_index)
    (Rendering|Debug|DrawDebugSphere (Math|Vector|MakeVector (Math|Conversions|ToFloat(Integer) (* _index 222)) 0.0 2e+02) 111.0 12 (Math|Color|Lerp(LinearColor) "(R=1.000000,G=0.070127,B=0.000000,A=1.000000)" "(R=0.000000,G=0.070262,B=1.000000,A=1.000000)" (/ (Math|Conversions|ToFloat(Integer) _index) (Math|Conversions|ToFloat(Integer) _last_index))) _duration 2.0))
  (Utilities|FlowControl|Delay (+ _duration 1.0))
  (CallFunction|ShowNodes) ; This is a GOTO lol
)

(fn ConstructionScript)