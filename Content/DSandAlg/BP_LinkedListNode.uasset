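; Linked list node actor that demonstrates list traversal and visualizes it in the world with debug drawing.
; getlength counts nodes with an iterative walk along NextNode, prints the total, then starts PingNode.
; PingNode prints and draws an index-tinted sphere, then after delays draws a line to the next node and pings it, chaining to the tail.
; It also calls GetLengthRecursive but discards the result, taking Length from EndNode's Index when valid.
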(event Custom|Ping%20Node
  (bind _nextnode (Variables|Default|GetnextNode))
  (bind _index (Variables|Default|Getindex))
  (bind _returnvalue (Math|Conversions|ToFloat(Integer) _index))
  (bind _returnvalue_2 (/ _returnvalue 1e+02))
  (bind _returnvalue_3 (Math|Color|Lerp(LinearColor) "(R=1.000000,G=0.624797,B=0.000000,A=1.000000)" "(R=0.010856,G=1.000000,B=0.000000,A=1.000000)" _returnvalue_2))
  (CallFunction|GetLengthRecursive (Variables|Default|GetnextNode))
  (bind _endnode (Variables|Default|GetEndNode)
    (:then
      (Variables|Default|SetLength (Variables|BP_LinkedListNode_C|Getindex _endnode)))
    (:else
      _))
  (Development|PrintString (Utilities|String|Append "pinging node " (Utilities|String|ToString(Integer) (Variables|Default|Getindex)) " of " (Utilities|String|ToString(Integer) (Variables|Default|GetLength))) true true _returnvalue_3 22.0)
  (Rendering|Debug|DrawDebugSphere (Transformation|GetActorLocation) 5e+01 6 _returnvalue_3 2.0 6.0)
  (Utilities|FlowControl|Delay (Variables|Default|Getdelay%20duration))
  (Utilities|IsValid _nextnode
    (:Is%20Valid
      (Rendering|Debug|DrawDebugLine (Transformation|GetActorLocation) (Transformation|GetActorLocation _nextnode) "(R=1.000000,G=0.000000,B=0.165793,A=1.000000)" 2.0 3.0)
      (Utilities|FlowControl|Delay (Variables|Default|Getdelay%20duration))
      (CallFunction|PingNode _nextnode))
    (:Is%20Not%20Valid
      (Development|PrintString "Done Pinging!"))))

(event Custom|get%20length
  (bind _length (Variables|Default|GetLength))
  (bind _output_get (Variables|Default|SettempNode (Variables|Default|GetnextNode)))
  (while (Utilities|IsValid (Variables|BP_LinkedListNode_C|GetnextNode _output_get))
    (Math|Integer|IncrementInt _length
      (:%20%20
        (Variables|Default|SettempNode (Variables|BP_LinkedListNode_C|GetnextNode (Variables|Default|GettempNode))) ; set the temp node to the next\nnode in the list
      )))
  (Development|PrintString (Utilities|String|Append "There are " (Utilities|String|ToString(Integer) _length) " nodes in the list"))
  (CallFunction|PingNode))

(fn ConstructionScript)

(fn GetLengthRecursive
  (params (head :type BP%20Linked%20List%20Node%20Object%20Reference))
  (Utilities|IsValid head
    (:Is%20Valid
      ;[1 1 1] i can skip the addition if I am returning the end node.
      (bind _length (CallFunction|GetLengthRecursive (Variables|BP_LinkedListNode_C|GetnextNode head))) ; head->next is in the parameter
      (return (+ _length 1) 0))
    (:Is%20Not%20Valid
      (Development|PrintString "tell everyone what the actual length is")
      (return 0 self))))