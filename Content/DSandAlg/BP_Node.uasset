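; BP_Node is a tree node actor that visualizes a level-by-level search for a goal node using timed debug spheres.
; The parentless root draws a blue sphere and starts CheckKids, which steps through Kids via delay loops, marking non-goals red and the goal green.
; Without a goal among its children, a node triggers CheckKids on each child in staggered, overlapping fashion.
; Finding the goal halts only that node's search, not branches already running.
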(event Custom|Check%20Kids
  (Utilities|FlowControl|Delay 1.0 :!label _label)
  (Utilities|IsValid (Utilities|Array|Get(acopy) (Variables|Default|GetKids) (Variables|Default|Getkid%20Index))
    (:Is%20Valid
      (if (Variables|BP_Node_C|GetThisIsTheGoal (Utilities|Array|Get(acopy) (Variables|Default|GetKids) (Variables|Default|Getkid%20Index)))
        (Rendering|Debug|DrawDebugSphere (Transformation|GetActorLocation (Utilities|Array|Get(acopy) (Variables|Default|GetKids) (Variables|Default|Getkid%20Index))) 111.0 24 "(R=0.012622,G=1.000000,B=0.000000,A=1.000000)" 22.0 5.0) ; draw a ball around us.
        (else
          (Rendering|Debug|DrawDebugSphere (Transformation|GetActorLocation (Utilities|Array|Get(acopy) (Variables|Default|GetKids) (Variables|Default|Getkid%20Index))) 111.0 24 "(R=1.000000,G=0.041622,B=0.000000,A=1.000000)" 22.0 5.0) ; draw a ball around us.
          (Math|Integer|IncrementInt (Variables|Default|Getkid%20Index)
            (:%20%20
              (goto _label))))))
    (:Is%20Not%20Valid
      ;[1 1 1] we are done looking at our kids, let's have our kids look at our grandkids
      (Variables|Default|Setkid%20Index 0)
      (Utilities|FlowControl|Delay 1.0 :!label _label_2)
      (Utilities|IsValid (Utilities|Array|Get(acopy) (Variables|Default|GetKids) (Variables|Default|Getkid%20Index))
        (:Is%20Valid
          (CallFunction|CheckKids (Utilities|Array|Get(acopy) (Variables|Default|GetKids) (Variables|Default|Getkid%20Index)))
          (Math|Integer|IncrementInt (Variables|Default|Getkid%20Index)
            (:%20%20
              (goto _label_2))))))))

(event EventBeginPlay
  (Utilities|IsValid (Variables|Default|GetParent)
    (:Is%20Not%20Valid
      (Utilities|FlowControl|Delay 1.0)
      (Rendering|Debug|DrawDebugSphere (Transformation|GetActorLocation) 111.0 24 "(R=0.000000,G=0.040319,B=1.000000,A=1.000000)" 22.0 5.0) ; draw a ball around us.
      (CallFunction|CheckKids))))

(fn ConstructionScript)