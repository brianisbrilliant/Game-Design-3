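; Node manager actor for a data-structures demo that spawns tree and linked-list node actors in the world.
; BeginPlay spawns a root BP_TreeNode and has it spawn four children.
; A self-calling event with a delay builds a doubly linked list at random offsets from the tail, but its setup is disconnected.
; A Space debug key calls GetLength on FirstNode, which only that unused setup assigns.
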(event Custom|Create%20new%20Node
  (bind _index (Variables|Default|GetIndex))
  (bind _returnvalue (Game|SpawnActorfromClass "/Game/DSandAlg/BP_LinkedListNode.BP_LinkedListNode_C" (Math|Transform|MakeTransform (Math|Random|RandomPointinBoundingBox (Transformation|GetActorLocation (Variables|Default|GetLastNode)) "1000.000000,1000.000000,100.000000") "0, 0, 0" "1.000000,1.000000,1.000000") "Undefined" "MultiplyWithRoot" 0 0))
  (Variables|/Game/DSandAlg/BP_LinkedListNode.BP_LinkedListNode_C|SetnextNode (Variables|Default|GetLastNode) _returnvalue) ; setting this new node to be the "next node"
  (Variables|/Game/DSandAlg/BP_LinkedListNode.BP_LinkedListNode_C|Setindex _returnvalue _index)
  (Math|Integer|IncrementInt _index
    (:%20%20
      (Variables|/Game/DSandAlg/BP_LinkedListNode.BP_LinkedListNode_C|SetprevNode _returnvalue (Variables|Default|GetLastNode)) ; setting the last node to be this node's \nprevious node.
      (Variables|Default|SetLastNode _returnvalue) ; Setting this new node to be the\nlast node
      (Utilities|FlowControl|Delay 1.0)
      (if (< (Variables|Default|GetIndex) 5)
        (CallFunction|CreateNewNode)))))

(event EventBeginPlay
  (Utilities|FlowControl|Sequence
    (:then_1
      (bind _returnvalue (Game|SpawnActorfromClass "/Game/DSandAlg/BP_TreeNode.BP_TreeNode_C" (Math|Transform|MakeTransform "0.000000,0.000000,300.000000" "0, 0, 0" "1.000000,1.000000,1.000000") "Undefined" "MultiplyWithRoot" 0 0))
      (Default|SpawnChildren _returnvalue "0.000000,0.000000,300.000000" 4))))

(event Input|KeyboardEvents|DebugKeySpaceBar
  (params (Key :type Key%20Structure :default "None") (ActionValue :type Input%20Action%20Value%20Structure))
  (:Pressed
    (Development|PrintString "calling get length")
    (Default|GetLength (Variables|Default|GetFirstNode))))

(fn ConstructionScript)