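; BP_TreeNode is a debug-visualized tree node actor that recursively spawns a randomly placed tree of itself.
; SpawnChildren records the parent, then spawns nodes with delays, storing each and recursing with one fewer kid.
; Spawn positions are scaled random unit vectors not offset from the parent.
; Each node draws a debug box, with lines from the passed ParentLocation to new nodes, colored by kid count.
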(event Custom|spawn%20children
  (params (parent%20location :type Vector) (total%20Kids :type Integer) (Parent :type BP%20Tree%20Node%20Object%20Reference))
  (Utilities|Array|Add (Variables|Default|GetParentArray) Parent)
  (Utilities|FlowControl|Delay (Variables|Default|Getdelay%20duration))
  (for _index (range 0 total%20Kids)
    (bind _returnvalue (Game|SpawnActorfromClass "BP_TreeNode_C" (Math|Transform|MakeTransform (* (Math|Random|RandomUnitVector) "400.000000,400.000000,50.000000") "0, 0, 0" "1.000000,1.000000,1.000000") "Undefined" "MultiplyWithRoot" 0 0))
    (Rendering|Debug|DrawDebugLine parent%20location (Transformation|GetActorLocation _returnvalue) (Utilities|Select :Index total%20Kids :Option%200 "" :Option%201 "(R=1.000000,G=0.069814,B=0.000000,A=1.000000)" :Option%202 "(R=0.000000,G=0.190921,B=1.000000,A=1.000000)" :Option%203 "(R=0.000000,G=1.000000,B=0.134206,A=1.000000)" :Option%204 "(R=1.000000,G=0.905656,B=0.000000,A=1.000000)" :Option%205 "(R=0.000000,G=1.000000,B=0.934435,A=1.000000)" :Option%206 "(R=1.000000,G=0.000000,B=0.875875,A=1.000000)") 22.0 2.0)
    (Utilities|Array|Add (Variables|Default|GetChildArray) _returnvalue)
    (Utilities|FlowControl|Delay (Variables|Default|Getdelay%20duration))
    (CallFunction|SpawnChildren _returnvalue (Transformation|GetActorLocation) (- total%20Kids 1) self)))

(event EventBeginPlay
  (Rendering|Debug|DrawDebugBox (Transformation|GetActorLocation) "22.000000,22.000000,22.000000" "(R=1.000000,G=0.435712,B=0.133961,A=1.000000)" "0, 0, 0" 22.0 4.0))

(fn ConstructionScript)