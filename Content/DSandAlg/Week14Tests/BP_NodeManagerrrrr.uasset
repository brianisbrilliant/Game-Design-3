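; Node manager actor that grows an endless doubly linked list of BP_NodeInClass actors in the level.
; BeginPlay spawns the first node at the manager's location, then SpawnNewNode re-calls itself after a short delay with no stop condition.
; Each new node spawns randomly in a box around the last, gets an incrementing index, and is linked through NextNode and PrevNode.
; DrawPath is an empty stub noted for Spacebar-triggered link creation.
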(event Custom|SpawnNewNode
  (bind _nodeindex (Variables|Default|GetNodeIndex))
  (Development|PrintString "Spawning a new node!")
  (bind _returnvalue (Game|SpawnActorfromClass "/Game/DSandAlg/Week14Tests/BP_NodeInClass.BP_NodeInClass_C" (Math|Transform|MakeTransform (Math|Random|RandomPointinBoundingBox (Transformation|GetActorLocation (Variables|Default|GetLastNode)) "500.000000,500.000000,500.000000") "0, 0, 0" "1.000000,1.000000,1.000000") "Undefined" "MultiplyWithRoot" 0 0))
  (Variables|/Game/DSandAlg/Week14Tests/BP_NodeInClass.BP_NodeInClass_C|SetIndex _returnvalue _nodeindex)
  (Math|Integer|IncrementInt _nodeindex
    (:%20%20
      (Variables|/Game/DSandAlg/Week14Tests/BP_NodeInClass.BP_NodeInClass_C|SetNextNode (Variables|Default|GetLastNode) _returnvalue) ; set the "next node"\non the first node.
      (Variables|/Game/DSandAlg/Week14Tests/BP_NodeInClass.BP_NodeInClass_C|SetPrevNode _returnvalue (Variables|Default|GetLastNode)) ; set the "previous node"\non this new node.
      (Variables|Default|SetLastNode _returnvalue) ; set the managers "Last Node"\nto be this new Node
      (Utilities|FlowControl|Delay 0.5)
      (CallFunction|SpawnNewNode))))

(event Custom|Draw%20Path)

(event EventBeginPlay
  (bind _nodeindex (Variables|Default|GetNodeIndex))
  (bind _returnvalue (Game|SpawnActorfromClass "/Game/DSandAlg/Week14Tests/BP_NodeInClass.BP_NodeInClass_C" (Math|Transform|MakeTransform (Transformation|GetActorLocation) "0, 0, 0" "1.000000,1.000000,1.000000") "Undefined" "MultiplyWithRoot" 0 0))
  (Variables|Default|SetLastNode _returnvalue)
  (Variables|/Game/DSandAlg/Week14Tests/BP_NodeInClass.BP_NodeInClass_C|SetIndex _returnvalue _nodeindex)
  (Math|Integer|IncrementInt _nodeindex
    (:%20%20
      (CallFunction|SpawnNewNode))))

(fn ConstructionScript)