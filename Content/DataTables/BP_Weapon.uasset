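; BP_Weapon is a weapon Blueprint with a mesh, a damage range, and text showing its weapon type, elemental type and damage.
; A randomize event adds small random increments to the current min and max damage, then refreshes the text and mesh.
; The mesh comes from a single WeaponMesh variable, while a lookup into a mesh array by weapon type sits unused.
; Nothing in this file calls the randomize event.
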(event Custom|setMesh
  ;[1 1 1] Use a struct
  (Components|StaticMesh|SetStaticMesh (Variables|Default|GetWeaponBody) (Variables|Default|GetWeaponMesh)))

(event Custom|randomize%20values
  (bind _output_get (Variables|Default|SetMinDamage (+ (Variables|Default|GetMinDamage) (Math|Random|RandomInteger 2))))
  (Variables|Default|SetMaxDamage (+ _output_get (Math|Random|RandomIntegerinRange 1 4)))
  (CallFunction|UpdateText)
  (CallFunction|SetMesh))

(event Custom|UpdateText
  (Rendering|Components|TextRender|SetText (Variables|Default|GetTextWeaponType) (Utilities|Text|ToText(String) (Utilities|String|EnumtoString (Variables|Default|GetWeaponType))))
  (Rendering|Components|TextRender|SetText (Variables|Default|GetTextElemType) (Utilities|Text|ToText(String) (Utilities|String|EnumtoString (Variables|Default|GetElementalType))))
  (Rendering|Components|TextRender|SetText (Variables|Default|GetTextDmg) (Utilities|Text|ToText(String) (Utilities|String|Append (Utilities|String|ToString(Integer) (Variables|Default|GetMinDamage)) "-" (Utilities|String|ToString(Integer) (Variables|Default|GetMaxDamage))))))

(fn ConstructionScript)